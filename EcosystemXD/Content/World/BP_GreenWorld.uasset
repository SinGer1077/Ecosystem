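; BP_GreenWorld is a world Blueprint that builds a flat patch of grass ground when its CreateWorld event fires.
; CreateWorld spawns a plain Actor at its own transform and adds a ProceduralMeshComponent to it at runtime.
; A zero-height GenerateBoxMesh result fills a mesh section with collision, which then receives the M_Bush material.
; BeginPlay is disabled and the construction script only calls its parent.
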(event `self.CreateWorld`
  (`KismetSystemLibrary.PrintString` "Creating world of grass")
  (bind _returnvalue (`|SpawnActorFromClass` "/Script/Engine.Actor" (`self.GetTransform`) "AlwaysSpawn" "MultiplyWithRoot" self null))
  (bind _returnvalue_2 (`AddComponent|NODE_AddProceduralMeshComponent-0` :`self` _returnvalue))
  (set `self.PMC` _returnvalue_2)
  (bind (_vertices _triangles _normals _uvs _tangents) (`KismetProceduralMeshLibrary.GenerateBoxMesh` (300.0 300.0 0.0)))
  (`ProceduralMeshComponent.CreateMeshSection_LinearColor` :`self` (`self.PMC`) :`Vertices` _vertices :`Triangles` _triangles :`UV0` _uvs :`Tangents` _tangents :`bCreateCollision` true)
  (`KismetProceduralMeshLibrary.GetSectionFromProceduralMesh` null)
  (`PrimitiveComponent.SetMaterial` (`self.PMC`) 0 "/Game/StarterContent/Props/Materials/M_Bush.M_Bush"))

(fn `UserConstructionScript`
  (`parent.UserConstructionScript`))